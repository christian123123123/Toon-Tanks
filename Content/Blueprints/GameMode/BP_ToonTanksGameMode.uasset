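; Game mode for Toon Tanks that shows the start and game over screens and handles level progression.
; StartGame adds the start widget, while GameOver shows a win or loss message and waits briefly before changing level.
; A win increments the level index in BP_GameInstance and opens that entry from its level name list, with no bounds check.
; A loss opens Main and resets the index to zero.
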(event `self.StartGame`
  (bind _returnvalue (`|CreateWidget` "/Game/Blueprints/Widgets/WBP_StartGameWidget.WBP_StartGameWidget_C"))
  (`UserWidget.AddToViewport` _returnvalue 0))

(event `self.GameOver`
  (params (bWonGame :type Boolean))
  (bind _returnvalue (`|CreateWidget` "/Game/Blueprints/Widgets/WBP_GameOverWidget.WBP_GameOverWidget_C"))
  (`UserWidget.AddToViewport` _returnvalue 0)
  (set `TextBlock.Text` (select `bool` bWonGame :`false` "YOU LOST! GOING BACK TO LEVEL 1" :`true` "YOU WIN! LOADING NEXT LEVEL!" :!type "Text") (`/Game/Blueprints/Widgets/WBP_GameOverWidget.DisplayText` _returnvalue))
  (`KismetSystemLibrary.Delay` 3.0)
  (if bWonGame
    (bind _asbp_game_instance (cast `/Game/Blueprints/BP_GameInstance` (`GameplayStatics.GetGameInstance`)))
    (bind _result (`/Engine/EditorBlueprintResources/StandardMacros.IncrementInt` (`/Game/Blueprints/BP_GameInstance.CurrentLevelIndex` _asbp_game_instance))
      (:`  `
        (bind _asbp_game_instance_2 (cast `/Game/Blueprints/BP_GameInstance` (`GameplayStatics.GetGameInstance`)))
        (`GameplayStatics.OpenLevel` (`KismetStringLibrary.Conv_StringToName` (`|GetArrayItem` (`/Game/Blueprints/BP_GameInstance.LevelNames` _asbp_game_instance_2) _result)))))
    (else
      (`GameplayStatics.OpenLevel` "Main")
      (bind _asbp_game_instance_3 (cast `/Game/Blueprints/BP_GameInstance` (`GameplayStatics.GetGameInstance`)))
      (set `/Game/Blueprints/BP_GameInstance.CurrentLevelIndex` 0 _asbp_game_instance_3))))

(fn `UserConstructionScript`)